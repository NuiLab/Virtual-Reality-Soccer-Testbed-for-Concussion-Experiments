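; Teleport portal actor that sends the game to another level when something overlaps its capsule.
; The construction script shows the LevelName variable on a text render, which Tick rotates to face the player pawn.
; On overlap, a switch on LevelName plays a fade-out level sequence, waits for a fixed delay, then opens the matching hardcoded level (base, single-skill or combined Evade/Goal/Pass).
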(event `self.ReceiveTick`
  (params (DeltaSeconds :type "Float (single-precision)"))
  (`SceneComponent.K2_SetWorldRotation` (`self.TextRender`) (`KismetMathLibrary.FindLookAtRotation` (`self.K2_GetActorLocation`) (`self.K2_GetActorLocation` (`GameplayStatics.GetPlayerPawn` 0))) false false))

(event `self.Capsule.OnComponentBeginOverlap`
  (params (OverlappedComponent :type "PrimitiveComponent Object Reference") (OtherActor :type "Actor Object Reference") (OtherComp :type "PrimitiveComponent Object Reference") (OtherBodyIndex :type Integer) (bFromSweep :type Boolean) (SweepResult :type "HitResult Structure (by ref)"))
  ;[0 1 1] FadeOut Sequence and Load Level
  (switch `string` (`KismetTextLibrary.Conv_TextToString` (`self.LevelName`))
    (:`Base Level`
      (bind (_outactor _returnvalue) (`LevelSequencePlayer.CreateLevelSequencePlayer` "/Game/Sequence/FadeOutSequence.FadeOutSequence"))
      (`MovieSceneSequencePlayer.Play` _returnvalue)
      (`KismetSystemLibrary.Delay` 1.38)
      (`GameplayStatics.OpenLevel` "Base_Level"))
    (:`Evade Level`
      (bind (_outactor_2 _returnvalue_2) (`LevelSequencePlayer.CreateLevelSequencePlayer` "/Game/Sequence/FadeOutSequence.FadeOutSequence"))
      (`MovieSceneSequencePlayer.Play` _returnvalue_2)
      (`KismetSystemLibrary.Delay` 1.38)
      (`GameplayStatics.OpenLevel` "1_Evade_Level"))
    (:`Goal Level`
      (bind (_outactor_3 _returnvalue_3) (`LevelSequencePlayer.CreateLevelSequencePlayer` "/Game/Sequence/FadeOutSequence.FadeOutSequence"))
      (`MovieSceneSequencePlayer.Play` _returnvalue_3)
      (`KismetSystemLibrary.Delay` 1.38)
      (`GameplayStatics.OpenLevel` "1_Goal_Level"))
    (:`Pass Level`
      (bind (_outactor_4 _returnvalue_4) (`LevelSequencePlayer.CreateLevelSequencePlayer` "/Game/Sequence/FadeOutSequence.FadeOutSequence"))
      (`MovieSceneSequencePlayer.Play` _returnvalue_4)
      (`KismetSystemLibrary.Delay` 1.38)
      (`GameplayStatics.OpenLevel` "1_Pass_Level"))
    (:`Evade+Goal Level`
      (bind (_outactor_5 _returnvalue_5) (`LevelSequencePlayer.CreateLevelSequencePlayer` "/Game/Sequence/FadeOutSequence.FadeOutSequence"))
      (`MovieSceneSequencePlayer.Play` _returnvalue_5)
      (`KismetSystemLibrary.Delay` 1.38)
      (`GameplayStatics.OpenLevel` "2_Evade+Goal_Level"))
    (:`Evade+Pass Level`
      (bind (_outactor_6 _returnvalue_6) (`LevelSequencePlayer.CreateLevelSequencePlayer` "/Game/Sequence/FadeOutSequence.FadeOutSequence"))
      (`MovieSceneSequencePlayer.Play` _returnvalue_6)
      (`KismetSystemLibrary.Delay` 1.38)
      (`GameplayStatics.OpenLevel` "2_Evade+Pass_Level"))))

(fn `UserConstructionScript`
  (`TextRenderComponent.K2_SetText` (`self.TextRender`) (`self.LevelName`)))