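; Still_MaleTargets is a short-lived soccer pass target that detects when the ball reaches it.
; An overlap on CircleBounds with an actor whose display name contains "SoccerBall" sets the pass success count to 2 and saves it to a text file.
; Four seconds after BeginPlay, it records that count in the game state's SuccessfulPasses and destroys itself.
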(event `self.ReceiveBeginPlay`
  ;[1 0 0] Destroy after a set amount of time
  (`KismetSystemLibrary.Delay` 4.0)
  (bind _assoccer_game_state (cast `/Game/Soccer_GameState` (`GameplayStatics.GetGameState`)))
  (bind _successful_passes (`/Game/Soccer_GameState.Successful_Passes` _assoccer_game_state))
  (`BlueprintMapLibrary.Map_Add` _successful_passes (`BlueprintMapLibrary.Map_Length` _successful_passes) (`self.Pass Success Count`))
  (`self.K2_DestroyActor`))

(event `self.Circle Bounds.OnComponentBeginOverlap`
  (params (OverlappedComponent :type "PrimitiveComponent Object Reference") (OtherActor :type "Actor Object Reference") (OtherComp :type "PrimitiveComponent Object Reference") (OtherBodyIndex :type Integer) (bFromSweep :type Boolean) (SweepResult :type "HitResult Structure (by ref)"))
  (if (`KismetStringLibrary.Contains` (`KismetSystemLibrary.GetDisplayName` OtherActor) "SoccerBall")
    (set `self.Pass Success Count` 2)
    (`RWTxtFile.SaveTxt` (`KismetStringLibrary.Conv_IntToString` (`self.Pass Success Count`)) (`self.File Name`))))

(fn `UserConstructionScript`)