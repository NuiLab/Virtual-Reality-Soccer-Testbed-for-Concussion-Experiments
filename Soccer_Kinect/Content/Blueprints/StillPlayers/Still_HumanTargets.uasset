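; Still human pass target for a soccer game that destroys itself four seconds after spawning.
; On BeginPlay it copies the successful pass count from Soccer_GameState.
; When an actor with SoccerBall in its name enters CircleBounds, it increments that count and saves it to a text file.
; It then sets the game state's SuccessfulPasses, but to an empty value rather than the new count.
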(event `self.ReceiveBeginPlay`
  ;[1 0 0] Destroy after a set amount of time
  (bind _assoccer_game_state (cast `/Game/Soccer_GameState` (`GameplayStatics.GetGameState`)))
  (set `self.Pass Success Count` (`.Successful_Passes` (`/Game/Soccer_GameState.Successful_Passes` _assoccer_game_state)))
  (`KismetSystemLibrary.Delay` 4.0)
  (`self.K2_DestroyActor`))

(event `self.Circle Bounds.OnComponentBeginOverlap`
  (params (OverlappedComponent :type "PrimitiveComponent Object Reference") (OtherActor :type "Actor Object Reference") (OtherComp :type "PrimitiveComponent Object Reference") (OtherBodyIndex :type Integer) (bFromSweep :type Boolean) (SweepResult :type "HitResult Structure (by ref)"))
  (bind _pass_success_count (`self.Pass Success Count`))
  (if (`KismetStringLibrary.Contains` (`KismetSystemLibrary.GetDisplayName` OtherActor) "SoccerBall")
    (`/Engine/EditorBlueprintResources/StandardMacros.IncrementInt` (`self.Pass Success Count`)
      (:`  `
        (`RWTxtFile.SaveTxt` (`KismetStringLibrary.Conv_IntToString` _pass_success_count) (`self.File Name`))
        (bind _assoccer_game_state (cast `/Game/Soccer_GameState` (`GameplayStatics.GetGameState`)))
        (set `/Game/Soccer_GameState.Successful_Passes` _ _pass_success_count _assoccer_game_state)))))

(fn `UserConstructionScript`)