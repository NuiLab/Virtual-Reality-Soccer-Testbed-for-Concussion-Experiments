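; Dummy actor that slides along its local negative X axis and removes itself once it passes a fixed world boundary.
; While ShouldMove is set, Tick applies an unswept local offset scaled by Speed and delta time.
; When world X drops below the limit, it calls Expired, which is empty in this graph, then destroys the actor.
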(event `self.ReceiveTick`
  (params (DeltaSeconds :type "Float (single-precision)"))
  (if (`self.shouldMove`)
    (`self.K2_AddActorLocalOffset` (`KismetMathLibrary.MakeVector` (* DeltaSeconds (* (`self.speed`) -1.0))))
    (if (not (>= (.x (`self.K2_GetActorLocation`)) -500.0))
      (`self.expired`)
      (`self.K2_DestroyActor`))))

(event `expired`)

(fn `UserConstructionScript`)