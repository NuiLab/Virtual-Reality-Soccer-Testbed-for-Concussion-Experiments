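; Trigger circle actor that starts a level change when its capsule is overlapped, and also visualizes the Oculus play area.
; A name-matched overlapping component, gated by the game instance's EnableCollision flag, plays a fade-out sequence, then after a delay clears the flag and opens the LoadLevel map.
; Tick draws the boundary's points and edges as debug shapes.
; Unwired logic would move the root to the average of those points.
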(event `self.ReceiveBeginPlay`)

(event `self.Capsule.OnComponentBeginOverlap`
  (params (OverlappedComponent :type "PrimitiveComponent Object Reference") (OtherActor :type "Actor Object Reference") (OtherComp :type "PrimitiveComponent Object Reference") (OtherBodyIndex :type Integer) (bFromSweep :type Boolean) (SweepResult :type "HitResult Structure (by ref)"))
  (bind _assoccer_game_instance (cast `/Game/Soccer_GameInstance` (`GameplayStatics.GetGameInstance`) :!pure true))
  (if (`KismetStringLibrary.Contains` (`KismetSystemLibrary.GetDisplayName` OtherComp) "TriggerCollision2397" true)
    (if (`/Game/Soccer_GameInstance.EnableCollision` (cast `/Game/Soccer_GameInstance` (`GameplayStatics.GetGameInstance`) :!pure true))
      (bind (_outactor _returnvalue) (`LevelSequencePlayer.CreateLevelSequencePlayer` "/Game/Sequence/FadeOutSequence.FadeOutSequence"))
      (`MovieSceneSequencePlayer.Play` _returnvalue)
      (`KismetSystemLibrary.Delay` 1.38)
      (set `/Game/Soccer_GameInstance.EnableCollision` false _assoccer_game_instance)
      (`GameplayStatics.OpenLevel` (`/Game/Soccer_GameInstance.LoadLevel` _assoccer_game_instance)))))

(event `self.ReceiveTick`
  (params (DeltaSeconds :type "Float (single-precision)"))
  (bind _oculusboundary (`self.OculusBoundary`))
  (bind _returnvalue (`OculusBoundaryComponent.GetPlayAreaPoints` _oculusboundary))
  (bind _returnvalue_2 (`KismetArrayLibrary.Array_Length` _returnvalue))
  ;[1 1 1] Draw the play area
  (if (`OculusBoundaryComponent.IsOuterBoundaryDisplayed` _oculusboundary)
    _
    (else
      _))
  (for _index (range _returnvalue_2)
    (bind _item (`KismetArrayLibrary.Array_Get` _returnvalue _index))
    (`KismetSystemLibrary.DrawDebugPoint` _item 10.0 (struct :`G` 1.0 :`B` 0.08537 :`A` 1.0))
    (`KismetSystemLibrary.DrawDebugLine` _item (`KismetArrayLibrary.Array_Get` _returnvalue (mod (+ _index 1) _returnvalue_2)) (struct :`R` 1.0 :`G` 0.01492 :`A` 1.0) 0.0 1.0)))

(fn `UserConstructionScript`)