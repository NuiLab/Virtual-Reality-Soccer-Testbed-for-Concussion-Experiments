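; Four-section soccer goal door that marks one active section in clear glass and the others in red-tinted glass.
; Once the game state's EGBallTaken is set, Tick turns all sections red, waits three seconds, then highlights Section1 and cycles onward every TimeGap seconds.
; An overlap on the active section's box, meant for the ball but unfiltered, also advances the cycle and restarts the timer.
; ChangeMaterial handles the wrapping index and material swap.
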(event `self.Box1.OnComponentBeginOverlap`
  (params (OverlappedComponent :type "PrimitiveComponent Object Reference") (OtherActor :type "Actor Object Reference") (OtherComp :type "PrimitiveComponent Object Reference") (OtherBodyIndex :type Integer) (bFromSweep :type Boolean) (SweepResult :type "HitResult Structure (by ref)"))
  ;[1 0 0] Check if Ball enters the goal in any section
  (if (== (`self.LastSection`) 0)
    (`self.Change Material`)
    (set `self.LastSectionSwitchTime` (`GameplayStatics.GetRealTimeSeconds`) :!label _label)))

(event `self.ReceiveBeginPlay`
  ;[0 0.178 1] Initial material settings
  (`PrimitiveComponent.SetMaterial` (`self.Section_2`) 0 "/Game/StarterContent/Materials/M_Glass.M_Glass")
  (`PrimitiveComponent.SetMaterial` (`self.Section_3`) 0 "/Game/StarterContent/Materials/M_Glass.M_Glass")
  (`PrimitiveComponent.SetMaterial` (`self.Section_4`) 0 "/Game/StarterContent/Materials/M_Glass.M_Glass")
  (`PrimitiveComponent.SetMaterial` (`self.Section_1`) 0 "/Game/StarterContent/Materials/M_Glass.M_Glass"))

(event `self.Box2.OnComponentBeginOverlap`
  (params (OverlappedComponent :type "PrimitiveComponent Object Reference") (OtherActor :type "Actor Object Reference") (OtherComp :type "PrimitiveComponent Object Reference") (OtherBodyIndex :type Integer) (bFromSweep :type Boolean) (SweepResult :type "HitResult Structure (by ref)"))
  ;[1 0 0] Check if Ball enters the goal in any section
  (if (== (`self.LastSection`) 1)
    (`self.Change Material`)
    (goto _label)))

(event `self.Box3.OnComponentBeginOverlap`
  (params (OverlappedComponent :type "PrimitiveComponent Object Reference") (OtherActor :type "Actor Object Reference") (OtherComp :type "PrimitiveComponent Object Reference") (OtherBodyIndex :type Integer) (bFromSweep :type Boolean) (SweepResult :type "HitResult Structure (by ref)"))
  ;[1 0 0] Check if Ball enters the goal in any section
  (if (== (`self.LastSection`) 2)
    (`self.Change Material`)
    (goto _label)))

(event `self.ReceiveTick`
  (params (DeltaSeconds :type "Float (single-precision)"))
  (bind _assoccer_game_state (cast `/Game/Soccer_GameState` (`GameplayStatics.GetGameState`)))
  (if (`/Game/Soccer_GameState.EG BallTaken` _assoccer_game_state)
    (if (`self.Switch`)
      ;[0 1 0] Condition checks to change goal section
      (if (> (- (`GameplayStatics.GetRealTimeSeconds`) (`self.LastSectionSwitchTime`)) (`self.TimeGap`))
        ;[0 1 1] Call to funtion to Change section
        (set `self.LastSectionSwitchTime` (`GameplayStatics.GetRealTimeSeconds`))
        (`self.Change Material`))
      (else
        (`PrimitiveComponent.SetMaterial` (`self.Section_2`) 0 "/Game/StarterContent/Materials/M_Glass_Tinted_Red.M_Glass_Tinted_Red")
        (`PrimitiveComponent.SetMaterial` (`self.Section_3`) 0 "/Game/StarterContent/Materials/M_Glass_Tinted_Red.M_Glass_Tinted_Red")
        (`PrimitiveComponent.SetMaterial` (`self.Section_4`) 0 "/Game/StarterContent/Materials/M_Glass_Tinted_Red.M_Glass_Tinted_Red")
        (`PrimitiveComponent.SetMaterial` (`self.Section_1`) 0 "/Game/StarterContent/Materials/M_Glass_Tinted_Red.M_Glass_Tinted_Red")
        (`KismetSystemLibrary.Delay` 3.0)
        (set `self.LastSectionSwitchTime` (`GameplayStatics.GetRealTimeSeconds`))
        (`PrimitiveComponent.SetMaterial` (`self.Section_1`) 0 "/Game/StarterContent/Materials/M_Glass.M_Glass")
        (set `self.Switch` true)))))

(event `self.Box4.OnComponentBeginOverlap`
  (params (OverlappedComponent :type "PrimitiveComponent Object Reference") (OtherActor :type "Actor Object Reference") (OtherComp :type "PrimitiveComponent Object Reference") (OtherBodyIndex :type Integer) (bFromSweep :type Boolean) (SweepResult :type "HitResult Structure (by ref)"))
  ;[1 0 0] Check if Ball enters the goal in any section
  (if (== (`self.LastSection`) 3)
    (`self.Change Material`)
    (goto _label)))

(fn `Change Material`
  ;[0 1 1] Condition checks for switching goal section
  (bind _result (`/Engine/EditorBlueprintResources/StandardMacros.IncrementInt` (`self.LastSection`))
    (:`  `
      (if (> _result 3)
        (set `self.LastSection` 0))
      (switch `int` (`self.LastSection`)
        (:`0`
          ;[0 0.5 1] Change section
          (`PrimitiveComponent.SetMaterial` (`self.Section_1`) 0 "/Game/StarterContent/Materials/M_Glass.M_Glass")
          (`PrimitiveComponent.SetMaterial` (`self.Section_4`) 0 "/Game/StarterContent/Materials/M_Glass_Tinted_Red.M_Glass_Tinted_Red"))
        (:`1`
          (`PrimitiveComponent.SetMaterial` (`self.Section_2`) 0 "/Game/StarterContent/Materials/M_Glass.M_Glass")
          (`PrimitiveComponent.SetMaterial` (`self.Section_1`) 0 "/Game/StarterContent/Materials/M_Glass_Tinted_Red.M_Glass_Tinted_Red"))
        (:`2`
          (`PrimitiveComponent.SetMaterial` (`self.Section_3`) 0 "/Game/StarterContent/Materials/M_Glass.M_Glass")
          (`PrimitiveComponent.SetMaterial` (`self.Section_2`) 0 "/Game/StarterContent/Materials/M_Glass_Tinted_Red.M_Glass_Tinted_Red"))
        (:`3`
          (`PrimitiveComponent.SetMaterial` (`self.Section_4`) 0 "/Game/StarterContent/Materials/M_Glass.M_Glass")
          (`PrimitiveComponent.SetMaterial` (`self.Section_3`) 0 "/Game/StarterContent/Materials/M_Glass_Tinted_Red.M_Glass_Tinted_Red"))))))

(fn `UserConstructionScript`)