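; A game state Blueprint that counts player strikes and ends the run after five.
; Tick accumulates elapsed time, and add_strike registers a strike only if at least five seconds have passed since the last one.
; At the strike limit it saves the elapsed time to the "last" save slot and opens the startfield level.
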(event `self.ReceiveTick`
  (params (DeltaSeconds :type "Float (single-precision)"))
  (set `self.time` (+ DeltaSeconds (`self.time`))))

(event `add_strike`
  (if (>= (- (`self.time`) (`self.lastStrike`)) 5.0)
    (set `self.lastStrike` (`self.time`))
    (bind _output_get (set `self.strikes` (+ (`self.strikes`) 1)))
    (if (>= _output_get 5)
      (bind _returnvalue (`GameplayStatics.CreateSaveGameObject` "/Game/Blueprints/save.save_C"))
      (set `/Game/Blueprints/save.time` (`self.time`) _returnvalue)
      (`GameplayStatics.SaveGameToSlot` _returnvalue "last")
      (`GameplayStatics.OpenLevel` "startfield"))))

(fn `UserConstructionScript`)