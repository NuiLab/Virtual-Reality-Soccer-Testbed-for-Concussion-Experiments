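; A throwable football that BP_MotionController picks up and drops in a game that counts strikes.
; Pickup snaps it to the given component with physics off; Drop re-enables physics and applies spin torque.
; Hitting a dummy freezes it and starts a beeping tick countdown, which force-releases all controllers, then destroys it with a strike.
; Hitting Landscape also clears BallExists on the game state, adds a strike and destroys it.
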(event `self.ReceiveBeginPlay`)

(event `self.ReceiveTick`
  (params (DeltaSeconds :type "Float (single-precision)"))
  (if (`self.hot`)
    (bind _output_get (set `self.hotTicks` (+ (`self.hotTicks`) 1)))
    (if (>= _output_get 10)
      (bind _outactors (`GameplayStatics.GetAllActorsOfClass` "/Game/VirtualRealityBP/Blueprints/BP_MotionController.BP_MotionController_C")) ; This is a dirty, filthy hack.  Enjoy my shame.
      (for _array_element _outactors
        (`/Game/VirtualRealityBP/Blueprints/BP_MotionController.ReleaseActor` _array_element))
      (bind _asstate (cast `/Game/Blueprints/state` (`GameplayStatics.GetGameState`)))
      (set `/Game/Blueprints/state.ball_exists` false _asstate)
      (`/Game/Blueprints/state.add_strike` _asstate)
      (`AudioComponent.Play` (`self.negative`) 0.0)
      (`self.K2_DestroyActor`)
      (else
        (`AudioComponent.Play` (`self.beep`) 0.0)))))

(event `/Game/VirtualRealityBP/Blueprints/PickupActorInterface.Pickup`
  (params (AttachTo :type "SceneComponent Object Reference"))
  (bind _staticmeshcomponent (`self.StaticMeshComponent`))
  (`PrimitiveComponent.SetSimulatePhysics` (`self.StaticMeshComponent`) false)
  (`SceneComponent.K2_AttachToComponent` (`self.K2_GetRootComponent`) AttachTo "None" "SnapToTarget" "SnapToTarget" "KeepWorld" false)
  (`SceneComponent.K2_AddLocalRotation` _staticmeshcomponent (struct :`Roll` 90.0) false false)
  (`SceneComponent.K2_AddLocalOffset` _staticmeshcomponent (-5.0 -3.0 -7.0) false false))

(event `/Game/VirtualRealityBP/Blueprints/PickupActorInterface.Drop`
  (bind _staticmeshcomponent (`self.StaticMeshComponent`))
  (`PrimitiveComponent.SetSimulatePhysics` (`self.StaticMeshComponent`) true)
  (`self.K2_DetachFromActor` "KeepWorld" "KeepWorld" "KeepWorld")
  (`PrimitiveComponent.SetPhysicsAngularVelocityInDegrees` _staticmeshcomponent (0.0 0.0 0.0) false "None")
  (`PrimitiveComponent.AddTorqueInDegrees` _staticmeshcomponent (`KismetMathLibrary.TransformDirection` (`self.GetTransform`) (0.0 100000.0 0.0)) "None" true))

(event `float`
  (`PrimitiveComponent.SetSimulatePhysics` (`self.StaticMeshComponent`) false)
  (set `self.hot` true))

(event `self.StaticMeshComponent.OnComponentHit`
  (params (HitComponent :type "PrimitiveComponent Object Reference") (OtherActor :type "Actor Object Reference") (OtherComp :type "PrimitiveComponent Object Reference") (NormalImpulse :type "Vector Structure") (Hit :type "HitResult Structure (by ref)"))
  (cast `/Game/Blueprints/dummy` OtherActor
    (:`then`
      (`self.float`))
    (:`CastFailed`
      (cast `Landscape` OtherActor)
      (bind _asstate (cast `/Game/Blueprints/state` (`GameplayStatics.GetGameState`)))
      (set `/Game/Blueprints/state.ball_exists` false _asstate)
      (`AudioComponent.Play` (`self.negative`) 0.0)
      (`/Game/Blueprints/state.add_strike` _asstate)
      (`self.K2_DestroyActor`))))

(fn `UserConstructionScript`)