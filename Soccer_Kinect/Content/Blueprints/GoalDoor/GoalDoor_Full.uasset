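; GoalDoor is a soccer goal trigger that logs scored and timed-out attempts to Soccer_GameState.
; Any overlap on Box1, with no check on the overlapping actor, records a success code, increments SuccessfulGoals and restarts the attempt timer.
; Unless KillInstances is set, Tick holds the timer reset while GoalStartSwitching is 1, then at higher values logs a different code whenever TimeGap elapses without a goal.
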(event `self.Box1.OnComponentBeginOverlap`
  (params (OverlappedComponent :type "PrimitiveComponent Object Reference") (OtherActor :type "Actor Object Reference") (OtherComp :type "PrimitiveComponent Object Reference") (OtherBodyIndex :type Integer) (bFromSweep :type Boolean) (SweepResult :type "HitResult Structure (by ref)"))
  ;[1 0 0] Check if Ball enters the goal in any section
  (bind _assoccer_game_state (cast `/Game/Soccer_GameState` (`GameplayStatics.GetGameState`)))
  (bind _goal_attempts (`/Game/Soccer_GameState.Goal_Attempts` _assoccer_game_state))
  (`BlueprintMapLibrary.Map_Add` _goal_attempts (`BlueprintMapLibrary.Map_Length` _goal_attempts) 2)
  (`/Engine/EditorBlueprintResources/StandardMacros.IncrementInt` (`/Game/Soccer_GameState.Successful_Goals` _assoccer_game_state)
    (:`  `
      (set `self.LastBallSpawnTime` (`GameplayStatics.GetRealTimeSeconds`)))))

(event `self.ReceiveTick`
  (params (DeltaSeconds :type "Float (single-precision)"))
  (bind _assoccer_game_state (cast `/Game/Soccer_GameState` (`GameplayStatics.GetGameState`) :!pure true))
  (bind _goal_start_switching (`/Game/Soccer_GameState.Goal Start Switching` _assoccer_game_state))
  (if (not (`/Game/Soccer_GameState.Kill Instances` _assoccer_game_state))
    (if (> _goal_start_switching 0)
      (if (== _goal_start_switching 1)
        (set `self.LastBallSpawnTime` (`GameplayStatics.GetRealTimeSeconds`))
        (elif (> (- (`GameplayStatics.GetRealTimeSeconds`) (`self.LastBallSpawnTime`)) (`self.TimeGap`))
          (set `self.LastBallSpawnTime` (`GameplayStatics.GetRealTimeSeconds`))
          (bind _assoccer_game_state_2 (cast `/Game/Soccer_GameState` (`GameplayStatics.GetGameState`)))
          (bind _goal_attempts (`/Game/Soccer_GameState.Goal_Attempts` _assoccer_game_state_2))
          (`BlueprintMapLibrary.Map_Add` _goal_attempts (`BlueprintMapLibrary.Map_Length` _goal_attempts) 1))))))

(fn `UserConstructionScript`)