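; Scoreboard for a five-attempt soccer passing level that shows a minutes:seconds clock and each attempt's result.
; Every Tick it looks up the current Hits index in Soccer_GameState's PassAttempts, marks that paired score text green "0" or red "X", then advances.
; The fifth result sets KillInstances without advancing Hits: a "0" quits the game, while an "X" plays a fade-out sequence and opens GameOver_Level.
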(event `self.ReceiveTick`
  (params (DeltaSeconds :type "Float (single-precision)"))
  (bind _returnvalue (`GameplayStatics.GetTimeSeconds`))
  (bind _returnvalue_2 (`KismetTextLibrary.Conv_StringToText` "0"))
  (bind _returnvalue_3 (`KismetTextLibrary.Conv_StringToText` "X"))
  (bind _score_2 (`self.Score 2`))
  (bind _score_3 (`self.Score 3`))
  (bind _score_4 (`self.Score 4`))
  (bind _score_5 (`self.Score 5`))
  (bind _score_1 (`self.Score 1`))
  (bind _score_2_2 (`self.Score 2`))
  (bind _score_3_2 (`self.Score 3`))
  (bind _score_4_2 (`self.Score 4`))
  (bind _score_5_2 (`self.Score 5`))
  (bind _score_1_2 (`self.Score 1`))
  (`TextRenderComponent.K2_SetText` (`self.Time`) (`KismetTextLibrary.Conv_StringToText` (`KismetStringLibrary.Concat_StrStr` (`KismetStringLibrary.Conv_IntToString` (`KismetMathLibrary.FFloor` (/ _returnvalue 60.0))) ":" (`KismetStringLibrary.Right` (`KismetStringLibrary.Concat_StrStr` "0" (`KismetStringLibrary.Conv_IntToString` (`KismetMathLibrary.FFloor` (mod _returnvalue 60.0)))) 2))))
  (bind _assoccer_game_state (cast `/Game/Soccer_GameState` (`GameplayStatics.GetGameState`)))
  (bind _pass_attempts (`/Game/Soccer_GameState.Pass_Attempts` _assoccer_game_state))
  (if (> (`BlueprintMapLibrary.Map_Length` _pass_attempts) 0)
    (bind _value (`BlueprintMapLibrary.Map_Find` _pass_attempts (`self.Hits`)))
    (if (== _value 2)
      (switch `int` (`self.Hits`)
        (:`0`
          (`TextRenderComponent.K2_SetText` _score_1 _returnvalue_2)
          (`TextRenderComponent.SetTextRenderColor` _score_1 (`KismetMathLibrary.Conv_LinearColorToColor` (struct :`G` 1.0 :`A` 1.0)))
          (`TextRenderComponent.K2_SetText` (`self.BScore 1`) _returnvalue_2)
          (`/Engine/EditorBlueprintResources/StandardMacros.IncrementInt` (`self.Hits`) :!label _label))
        (:`1`
          (`TextRenderComponent.K2_SetText` _score_2 _returnvalue_2)
          (`TextRenderComponent.SetTextRenderColor` _score_2 (`KismetMathLibrary.Conv_LinearColorToColor` (struct :`G` 1.0 :`A` 1.0)))
          (`TextRenderComponent.K2_SetText` (`self.BScore 2`) _returnvalue_2)
          (goto _label))
        (:`2`
          (`TextRenderComponent.K2_SetText` _score_3 _returnvalue_2)
          (`TextRenderComponent.SetTextRenderColor` _score_3 (`KismetMathLibrary.Conv_LinearColorToColor` (struct :`G` 1.0 :`A` 1.0)))
          (`TextRenderComponent.K2_SetText` (`self.BScore 3`) _returnvalue_2)
          (goto _label))
        (:`3`
          (`TextRenderComponent.K2_SetText` _score_4 _returnvalue_2)
          (`TextRenderComponent.SetTextRenderColor` _score_4 (`KismetMathLibrary.Conv_LinearColorToColor` (struct :`G` 1.0 :`A` 1.0)))
          (`TextRenderComponent.K2_SetText` (`self.BScore 4`) _returnvalue_2)
          (goto _label))
        (:`4`
          (`TextRenderComponent.K2_SetText` _score_5 _returnvalue_2)
          (`TextRenderComponent.SetTextRenderColor` _score_5 (`KismetMathLibrary.Conv_LinearColorToColor` (struct :`G` 1.0 :`A` 1.0)))
          (`TextRenderComponent.K2_SetText` (`self.BScore 5`) _returnvalue_2)
          (set `/Game/Soccer_GameState.Kill Instances` true (cast `/Game/Soccer_GameState` (`GameplayStatics.GetGameState`) :!pure true))
          (`KismetSystemLibrary.QuitGame` null "Quit")))
      (elif (== _value 1)
        (switch `int` (`self.Hits`)
          (:`0`
            (`TextRenderComponent.K2_SetText` _score_1_2 _returnvalue_3)
            (`TextRenderComponent.SetTextRenderColor` _score_1_2 (`KismetMathLibrary.Conv_LinearColorToColor` (struct :`R` 1.0 :`A` 1.0)))
            (`TextRenderComponent.K2_SetText` (`self.BScore 1`) _returnvalue_3)
            (`/Engine/EditorBlueprintResources/StandardMacros.IncrementInt` (`self.Hits`) :!label _label_2))
          (:`1`
            (`TextRenderComponent.K2_SetText` _score_2_2 _returnvalue_3)
            (`TextRenderComponent.SetTextRenderColor` _score_2_2 (`KismetMathLibrary.Conv_LinearColorToColor` (struct :`R` 1.0 :`A` 1.0)))
            (`TextRenderComponent.K2_SetText` (`self.BScore 2`) _returnvalue_3)
            (goto _label_2))
          (:`2`
            (`TextRenderComponent.K2_SetText` _score_3_2 _returnvalue_3)
            (`TextRenderComponent.SetTextRenderColor` _score_3_2 (`KismetMathLibrary.Conv_LinearColorToColor` (struct :`R` 1.0 :`A` 1.0)))
            (`TextRenderComponent.K2_SetText` (`self.BScore 3`) _returnvalue_3)
            (goto _label_2))
          (:`3`
            (`TextRenderComponent.K2_SetText` _score_4_2 _returnvalue_3)
            (`TextRenderComponent.SetTextRenderColor` _score_4_2 (`KismetMathLibrary.Conv_LinearColorToColor` (struct :`R` 1.0 :`A` 1.0)))
            (`TextRenderComponent.K2_SetText` (`self.BScore 4`) _returnvalue_3)
            (goto _label_2))
          (:`4`
            (`TextRenderComponent.K2_SetText` _score_5_2 _returnvalue_3)
            (`TextRenderComponent.SetTextRenderColor` _score_5_2 (`KismetMathLibrary.Conv_LinearColorToColor` (struct :`R` 1.0 :`A` 1.0)))
            (`TextRenderComponent.K2_SetText` (`self.BScore 5`) _returnvalue_3)
            (set `/Game/Soccer_GameState.Kill Instances` true (cast `/Game/Soccer_GameState` (`GameplayStatics.GetGameState`) :!pure true))
            (bind (_outactor _returnvalue_4) (`LevelSequencePlayer.CreateLevelSequencePlayer` "/Game/Sequence/FadeOutSequence.FadeOutSequence"))
            (`MovieSceneSequencePlayer.Play` _returnvalue_4)
            (`KismetSystemLibrary.Delay` 1.38)
            (`GameplayStatics.OpenLevel` "GameOver_Level")))))))

(fn `UserConstructionScript`)