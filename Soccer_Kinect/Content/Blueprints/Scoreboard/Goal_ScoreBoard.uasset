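; Goal scoreboard actor for a soccer game that displays elapsed time and a successful-goals-over-attempts score.
; Every Tick it formats game time as minutes and zero-padded seconds for the Time text.
; It also polls the Soccer_GameState Attempts map using its own attempt counter as key.
; A value of 2 counts a goal, 1 only refreshes the score, and both advance the counter.
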(event `self.ReceiveTick`
  (params (DeltaSeconds :type "Float (single-precision)"))
  (bind _returnvalue (`GameplayStatics.GetTimeSeconds`))
  (`TextRenderComponent.K2_SetText` (`self.Time`) (`KismetTextLibrary.Conv_StringToText` (`KismetStringLibrary.Concat_StrStr` (`KismetStringLibrary.Conv_IntToString` (`KismetMathLibrary.FFloor` (/ _returnvalue 60.0))) ":" (`KismetStringLibrary.Right` (`KismetStringLibrary.Concat_StrStr` "0" (`KismetStringLibrary.Conv_IntToString` (`KismetMathLibrary.FFloor` (mod _returnvalue 60.0)))) 2))))
  (bind _assoccer_game_state (cast `/Game/Soccer_GameState` (`GameplayStatics.GetGameState`)))
  (bind _attempts (`/Game/Soccer_GameState.Attempts` _assoccer_game_state))
  (if (> (`BlueprintMapLibrary.Map_Length` _attempts) 0)
    (bind _value (`BlueprintMapLibrary.Map_Find` _attempts (`self.Attempts`)))
    (if (== _value 2)
      (bind _result (`/Engine/EditorBlueprintResources/StandardMacros.IncrementInt` (`self.Successful Goal`))
        (:`  `
          (`TextRenderComponent.K2_SetText` (`self.Score`) (`KismetTextLibrary.Conv_StringToText` (`KismetStringLibrary.Concat_StrStr` (`KismetStringLibrary.Conv_IntToString` _result) "/" (`KismetStringLibrary.Conv_IntToString` (`self.Attempts`)))))
          (`/Engine/EditorBlueprintResources/StandardMacros.IncrementInt` (`self.Attempts`) :!label _label)))
      (elif (== _value 1)
        (`TextRenderComponent.K2_SetText` (`self.Score`) (`KismetTextLibrary.Conv_StringToText` (`KismetStringLibrary.Concat_StrStr` (`KismetStringLibrary.Conv_IntToString` (`self.Successful Goal`)) "/" (`KismetStringLibrary.Conv_IntToString` (`self.Attempts`)))))
        (goto _label)))))

(fn `UserConstructionScript`)