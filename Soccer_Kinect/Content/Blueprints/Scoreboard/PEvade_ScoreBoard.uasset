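; PEvade scoreboard that shows elapsed game time as minutes:seconds and tracks collisions, ending the game on the second.
; Tick polls Soccer_GameState.Collisions against a local Hits count, turning one score text red per collision.
; The second collision sets KillInstances, plays a fade-out sequence and opens GameOver_Level after a short delay.
; That branch never increments Hits, so it re-fires every tick until the level changes.
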(event `self.ReceiveTick`
  (params (DeltaSeconds :type "Float (single-precision)"))
  (bind _returnvalue (`GameplayStatics.GetTimeSeconds`))
  (`TextRenderComponent.K2_SetText` (`self.Time`) (`KismetTextLibrary.Conv_StringToText` (`KismetStringLibrary.Concat_StrStr` (`KismetStringLibrary.Conv_IntToString` (`KismetMathLibrary.FFloor` (/ _returnvalue 60.0))) ":" (`KismetStringLibrary.Right` (`KismetStringLibrary.Concat_StrStr` "0" (`KismetStringLibrary.Conv_IntToString` (`KismetMathLibrary.FFloor` (mod _returnvalue 60.0)))) 2))))
  (bind _assoccer_game_state (cast `/Game/Soccer_GameState` (`GameplayStatics.GetGameState`)))
  (bind _collisions (`/Game/Soccer_GameState.Collisions` _assoccer_game_state))
  (if (> _collisions (`self.Hits`))
    (switch `int` _collisions
      (:`1`
        (`TextRenderComponent.SetTextRenderColor` (`self.Score 3`) (`KismetMathLibrary.Conv_LinearColorToColor` (struct :`R` 1.0 :`A` 1.0)))
        (`/Engine/EditorBlueprintResources/StandardMacros.IncrementInt` (`self.Hits`)))
      (:`2`
        (`TextRenderComponent.SetTextRenderColor` (`self.Score 4`) (`KismetMathLibrary.Conv_LinearColorToColor` (struct :`R` 1.0 :`A` 1.0)))
        (set `/Game/Soccer_GameState.Kill Instances` true (cast `/Game/Soccer_GameState` (`GameplayStatics.GetGameState`) :!pure true))
        (bind (_outactor _returnvalue_2) (`LevelSequencePlayer.CreateLevelSequencePlayer` "/Game/Sequence/FadeOutSequence.FadeOutSequence"))
        (`MovieSceneSequencePlayer.Play` _returnvalue_2)
        (`KismetSystemLibrary.Delay` 1.38)
        (`GameplayStatics.OpenLevel` "GameOver_Level")))))

(fn `UserConstructionScript`)