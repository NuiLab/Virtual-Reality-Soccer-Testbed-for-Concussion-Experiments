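; Scoreboard for a soccer passing drill that shows elapsed time and successful passes out of attempts made.
; Each Tick refreshes the clock and polls the Soccer_GameState PassAttempts map for the current attempt's result, counting successes and updating the score.
; When the trial count is reached, it saves the success count to a text file, plays a fade-out sequence and opens the game-over level.
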(event `self.ReceiveTick`
  (params (DeltaSeconds :type "Float (single-precision)"))
  (bind _returnvalue (`GameplayStatics.GetTimeSeconds`))
  (`TextRenderComponent.K2_SetText` (`self.Time`) (`KismetTextLibrary.Conv_StringToText` (`KismetStringLibrary.Concat_StrStr` (`KismetStringLibrary.Conv_IntToString` (`KismetMathLibrary.FFloor` (/ _returnvalue 60.0))) ":" (`KismetStringLibrary.Right` (`KismetStringLibrary.Concat_StrStr` "0" (`KismetStringLibrary.Conv_IntToString` (`KismetMathLibrary.FFloor` (mod _returnvalue 60.0)))) 2))))
  (bind _assoccer_game_state (cast `/Game/Soccer_GameState` (`GameplayStatics.GetGameState`)))
  (bind _pass_attempts (`/Game/Soccer_GameState.Pass_Attempts` _assoccer_game_state))
  (if (> (`BlueprintMapLibrary.Map_Length` _pass_attempts) 0)
    (bind _value (`BlueprintMapLibrary.Map_Find` _pass_attempts (`self.Attempts`)))
    (if (== _value 2)
      (bind _result (`/Engine/EditorBlueprintResources/StandardMacros.IncrementInt` (`self.Successful Pass`))
        (:`  `
          (`TextRenderComponent.K2_SetText` (`self.Score`) (`KismetTextLibrary.Conv_StringToText` (`KismetStringLibrary.Concat_StrStr` (`KismetStringLibrary.Conv_IntToString` _result) "/" (`KismetStringLibrary.Conv_IntToString` (+ (`self.Attempts`) 1)))))
          (`/Engine/EditorBlueprintResources/StandardMacros.IncrementInt` (`self.Attempts`) :!label _label
            (:`  `
              (if (>= (`self.Attempts`) (`self.Number of Trials`))
                (`RWTxtFile.SaveTxt` (`KismetStringLibrary.Conv_IntToString` (`self.Successful Pass`)) (`self.File Name`))
                (bind (_outactor _returnvalue_2) (`LevelSequencePlayer.CreateLevelSequencePlayer` "/Game/Sequence/FadeOutSequence.FadeOutSequence"))
                (`MovieSceneSequencePlayer.Play` _returnvalue_2)
                (`KismetSystemLibrary.Delay` 1.38)
                (`GameplayStatics.OpenLevel` "GameOver_Level"))))))
      (elif (== _value 1)
        (`TextRenderComponent.K2_SetText` (`self.Score`) (`KismetTextLibrary.Conv_StringToText` (`KismetStringLibrary.Concat_StrStr` (`KismetStringLibrary.Conv_IntToString` (`self.Successful Pass`)) "/" (`KismetStringLibrary.Conv_IntToString` (+ (`self.Attempts`) 1)))))
        (goto _label)))))

(fn `UserConstructionScript`)