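; AI soccer player that charges to a preset end point once it sees a pawn, then destroys itself on arrival.
; On BeginPlay it caches the end point's world location and, after a short delay, shows its ball if SetBall is on and no ball exists.
; A BallExists flag in Soccer_GameState coordinates the ball between actors; players with SetBall on clear it before being destroyed.
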(event `self.ReceiveBeginPlay`
  ;[1 1 0] Set the end point
  (set `self.End_Position` (`SceneComponent.K2_GetComponentLocation` (`self.end position`)))
  ;[0 0.5344 1] Condition check for attaching ball to player
  (`KismetSystemLibrary.Delay` 0.2)
  (bind _assoccer_game_state (cast `/Game/Soccer_GameState` (`GameplayStatics.GetGameState`)))
  (if (and (not (`/Game/Soccer_GameState.Ball Exists` _assoccer_game_state)) (`self.Set Ball`))
    ;[1 0.186 1] Attach ball
    (`SceneComponent.SetVisibility` (`self.SoccerBall`) true false)
    (bind _assoccer_game_state_2 (cast `/Game/Soccer_GameState` (`GameplayStatics.GetGameState`)))
    (set `/Game/Soccer_GameState.Ball Exists` true _assoccer_game_state_2)))

(event `self.PawnSensing.OnSeePawn`
  (params (Pawn :type "Pawn Object Reference"))
  ;[1 0 0] Move the player to end point and destroy on success
  (`|AIMoveTo` self (`self.End_Position`) null
    (:`OnSuccess`
      (if (`self.Set Ball`)
        (bind _assoccer_game_state (cast `/Game/Soccer_GameState` (`GameplayStatics.GetGameState`)))
        (set `/Game/Soccer_GameState.Ball Exists` false _assoccer_game_state)
        (set `self.Set Ball` false))
      (`self.K2_DestroyActor`))))

(fn `UserConstructionScript`)